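; BP_TutorialMySpawner is an overlap-triggered spawner for BP_RunningEnemy that only acts during round 1.
; Each BP_MyCharacter overlap makes a weighted random roll until one succeeds, then HasBeenPassed blocks further spawns.
; The enemy spawns at StartingPoint and receives FinishLine as its Target.
; One of two monster spawn sounds then plays at random, located at the world origin rather than at the spawn.
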(event `self.ReceiveBeginPlay`
  (set `self.HasBeenPassed` false)
  (bind _asmy_game_instance (cast `/Game/Blueprints/MyGameInstance` (`GameplayStatics.GetGameInstance`))))

(event `self.ReceiveActorBeginOverlap`
  (params (OtherActor :type "Actor Object Reference"))
  (if (== (`/Game/Blueprints/MyGameInstance.Round` (stale `self.ReceiveBeginPlay` _asmy_game_instance)) 1)
    (cast `/Game/Blueprints/BP_MyCharacter` OtherActor)
    (`KismetSystemLibrary.PrintString` "Hello")
    (if (`self.HasBeenPassed`)
      _
      (elif (`KismetMathLibrary.RandomBoolWithWeight` (`self.RandomWeight`))
        (set `self.HasBeenPassed` true)
        (bind _returnvalue (`AIBlueprintHelperLibrary.SpawnAIFromClass` "/Game/Blueprints/BP_RunningEnemy.BP_RunningEnemy_C" null (`self.K2_GetActorLocation` (`self.StartingPoint`)) (struct) false null))
        (bind _asbp_running_enemy (cast `/Game/Blueprints/BP_RunningEnemy` _returnvalue))
        (set `RunningEnemy.Target` (`self.FinishLine`) _asbp_running_enemy)
        (if (`KismetMathLibrary.RandomBoolWithWeight` 0.5)
          (`GameplayStatics.PlaySoundAtLocation` "/Game/Sounds/Enemies/RunningEnemy/Monster_Spawn_1_Cue.Monster_Spawn_1_Cue" (0.0 0.0 0.0) (struct) 1.0 1.0 0.0 null null null null)
          (else
            (`GameplayStatics.PlaySoundAtLocation` "/Game/Sounds/Enemies/RunningEnemy/Monster_Spawn_2_Cue.Monster_Spawn_2_Cue" (0.0 0.0 0.0) (struct) 1.0 1.0 0.0 null null null null)))))))

(fn `UserConstructionScript`)