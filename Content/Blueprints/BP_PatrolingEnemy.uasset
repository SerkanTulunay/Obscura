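; Patrolling enemy character that walks between patrol points and catches the player on contact.
; Tick issues AI MoveTo toward the current point and, on success, advances to the next one, looping back to the first.
; Overlapping a player character who is not hiding reloads the current level.
; BeginPlay sets a slow walk speed, targets the first point and starts its audio.
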(event `self.ReceiveBeginPlay`
  (set `CharacterMovementComponent.MaxWalkSpeed` 100.0 (`self.CharacterMovement`))
  (set `self.Target` (`|GetArrayItem` (`self.PatrolPoints`)))
  (`AudioComponent.Play` (`self.Audio`) 0.0))

(event `self.ReceiveActorBeginOverlap`
  (params (OtherActor :type "Actor Object Reference"))
  (bind _asbp_my_character (cast `/Game/Blueprints/BP_MyCharacter` OtherActor))
  (if (not (`MyCharacter.bIsHiding` _asbp_my_character))
    (bind _returnvalue (`GameplayStatics.GetCurrentLevelName` true))
    (`GameplayStatics.OpenLevel` (`KismetStringLibrary.Conv_StringToName` _returnvalue))))

(event `self.ReceiveTick`
  (params (DeltaSeconds :type "Float (single-precision)"))
  (bind _patrolpoints (`self.PatrolPoints`))
  (bind _counter (`self.Counter`))
  (bind _returnvalue (+ _counter 1))
  (`|AIMoveTo` self (0.0 0.0 0.0) (`self.Target`)
    (:`OnSuccess`
      (if (>= _returnvalue (`KismetArrayLibrary.Array_Length` _patrolpoints))
        (set `self.Counter` 0)
        (else
          (set `self.Counter` _returnvalue)))
      (set `self.Target` (`|GetArrayItem` _patrolpoints _counter)))))

(fn `UserConstructionScript`)