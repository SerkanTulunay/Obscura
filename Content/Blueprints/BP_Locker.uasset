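; BP_Locker is a locker Blueprint that toggles its Audio component based on whether the player is hiding.
; BeginPlay caches the player as BP_MyCharacter, obtained through the character movement component's pawn owner.
; Every Tick polls that character's IsHiding flag, stopping the audio while true and otherwise restarting it from the beginning whenever it is not playing.
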(event `self.ReceiveBeginPlay`
  (bind _asbp_my_character (cast `/Game/Blueprints/BP_MyCharacter` (`PawnMovementComponent.GetPawnOwner` (`Character.CharacterMovement` (`GameplayStatics.GetPlayerCharacter` 0))))))

(event `self.ReceiveTick`
  (params (DeltaSeconds :type "Float (single-precision)"))
  (bind _audio (`self.Audio`))
  (if (`MyCharacter.bIsHiding` (stale `self.ReceiveBeginPlay` _asbp_my_character))
    (`AudioComponent.Stop` _audio)
    (elif (not (`AudioComponent.IsPlaying` _audio))
      (`AudioComponent.Play` _audio 0.0))))

(fn `UserConstructionScript`)