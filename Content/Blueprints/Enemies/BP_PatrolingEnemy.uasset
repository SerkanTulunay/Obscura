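; BP_PatrolingEnemy is an enemy that walks a looping route of patrol points and attacks the player at close range.
; Tick reissues AIMoveTo toward the current point, advancing on success, and checks player distance.
; In range, it plays a charge cue at world origin and waits before calling Attack, whose body is not shown.
; While attacking or stunned, it stops moving and fades out its audio.
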(event `self.ReceiveBeginPlay`
  (set `CharacterMovementComponent.MaxWalkSpeed` 100.0 (`self.CharacterMovement`))
  (set `self.Target` (`|GetArrayItem` (`self.PatrolPoints`))))

(event `self.ReceiveTick`
  (params (DeltaSeconds :type "Float (single-precision)"))
  (bind _counter (`self.Counter`))
  (bind _patrolpoints (`self.PatrolPoints`))
  (bind _audio (`self.Audio`))
  (bind _charactermovement (`self.CharacterMovement`))
  (bind _returnvalue (+ _counter 1))
  (if (not (`AudioComponent.IsPlaying` _audio))
    (`AudioComponent.Play` _audio 0.0))
  (if (or (`self.bIsAttacking`) (`self.bIsStunned`))
    (set `CharacterMovementComponent.MaxWalkSpeed` 0.0 _charactermovement)
    (`AudioComponent.AdjustVolume` (`self.Audio`) 0.5 0.0 "Linear")
    (else
      (set `CharacterMovementComponent.MaxWalkSpeed` 100.0 _charactermovement)
      (`AudioComponent.AdjustVolume` (`self.Audio`) 0.5 1.0 "Linear")))
  (`|AIMoveTo` self (0.0 0.0 0.0) (`self.Target`)
    (:`then`
      _)
    (:`OnSuccess`
      (if (>= _returnvalue (`KismetArrayLibrary.Array_Length` _patrolpoints))
        (set `self.Counter` 0)
        (else
          (set `self.Counter` _returnvalue)))
      (set `self.Target` (`|GetArrayItem` _patrolpoints _counter))))
  (if (<= (`KismetMathLibrary.Vector_Distance` (`self.K2_GetActorLocation`) (`self.K2_GetActorLocation` (`GameplayStatics.GetPlayerCharacter` 0))) 200.0)
    (if (and (!= (`self.bIsAttacking`) true) (!= (`self.bIsStunned`) true))
      (set `self.bIsAttacking` true)
      ;[1 1 1] Attacks player if possible
      (`GameplayStatics.PlaySoundAtLocation` "/Game/Sounds/NewFolder/Monster_Attack_Charge_Cue.Monster_Attack_Charge_Cue" (0.0 0.0 0.0) (struct) 1.0 1.0 0.0 null null null null)
      (`KismetSystemLibrary.Delay` 2.0)
      (`self.Attack`)
      (set `self.bIsAttacking` false))))

(fn `UserConstructionScript`)