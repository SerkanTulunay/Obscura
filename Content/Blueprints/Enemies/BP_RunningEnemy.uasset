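; A charging enemy that plays audio and pursues its Target, respawning any non-hiding player character it touches.
; Every tick it reads the audio volume and walk speed from settings and reissues an AI MoveTo toward the Target.
; On catching an exposed player, it also clears HasBeenPassed on its owning spawner and destroys itself, while hiding players are ignored on overlap.
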(event `self.ReceiveBeginPlay`
  (`AudioComponent.Play` (`self.Audio`) 0.0))

(event `self.ReceiveActorBeginOverlap`
  (params (OtherActor :type "Actor Object Reference"))
  (bind _asbp_my_character (cast `/Game/Blueprints/BP_MyCharacter` OtherActor))
  (if (not (`MyCharacter.bIsHiding` _asbp_my_character))
    (`MyCharacter.Respawn` _asbp_my_character)
    (bind _asbp_my_spawner (cast `/Game/Blueprints/Enemies/BP_MySpawner` (`self.GetOwner`)))
    (set `/Game/Blueprints/Enemies/BP_MySpawner.HasBeenPassed` false _asbp_my_spawner)
    (`self.K2_DestroyActor`)))

(event `self.ReceiveTick`
  (params (DeltaSeconds :type "Float (single-precision)"))
  (bind _returnvalue (`ObscuraSettings.GetSettings`))
  (bind _output_get (set `self.IdleVolume` (`ObscuraSettings.ChargingEnemyVolume` _returnvalue)))
  (`AudioComponent.SetVolumeMultiplier` (`self.Audio`) _output_get)
  (bind _output_get_2 (set `self.MoveSpeed` (`ObscuraSettings.ChargingEnemyMoveSpeed` _returnvalue)))
  (set `CharacterMovementComponent.MaxWalkSpeed` _output_get_2 (`self.CharacterMovement`))
  (`|AIMoveTo` self (0.0 0.0 0.0) (`self.Target`)))

(fn `UserConstructionScript`)