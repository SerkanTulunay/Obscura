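; BP_CryingVent is an enemy hazard that restarts the current level when the player lingers inside its box volume for too long.
; Tick raises Health, used as an exposure timer, while the player overlaps the box and drains it toward zero otherwise.
; Health drives the volume of one looping-or-not audio component as a warning, while a second plays from BeginPlay at unadjusted volume.
; Crossing the exposure threshold reopens the level by name.
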(event `self.ReceiveBeginPlay`
  (`AudioComponent.Play` (`self.Audio1`) 0.0)
  (`AudioComponent.Play` (`self.Audio2`) 0.0)
  (set `self.Health` 0.0))

(event `self.ReceiveActorBeginOverlap`
  (params (OtherActor :type "Actor Object Reference")))

(event `self.ReceiveTick`
  (params (DeltaSeconds :type "Float (single-precision)"))
  (bind _health (`self.Health`))
  (`AudioComponent.AdjustVolume` (`self.Audio1`) 0.0 (+ (/ (`self.Health`) 3.0) 0.001) "Linear")
  (if (`PrimitiveComponent.IsOverlappingActor` (`self.Box`) (`GameplayStatics.GetPlayerCharacter` 0))
    (set `self.Health` (+ (`self.Health`) DeltaSeconds))
    (if (> (`self.Health`) 10.0) :!label _label
      (bind _returnvalue (`GameplayStatics.GetCurrentLevelName` true))
      (`GameplayStatics.OpenLevel` (`KismetStringLibrary.Conv_StringToName` _returnvalue)))
    (elif (> _health 0.009)
      (set `self.Health` (- _health DeltaSeconds))
      (goto _label))))

(fn `UserConstructionScript`)