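; Enemy Blueprint that chases the player character and makes a charged attack at close range.
; Tick freezes movement while attacking or stunned, reissues AIMoveTo toward the player and checks distance right away, without waiting for arrival.
; In range, it plays a charge sound at the world origin, waits, then calls Attack, which is not defined here.
; GetStunned is an empty stub, and nothing here sets the stunned flag.
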(event `self.ReceiveBeginPlay`
  (set `CharacterMovementComponent.MaxWalkSpeed` 100.0 (`self.CharacterMovement`))
  (set `self.Target` (`GameplayStatics.GetPlayerCharacter` 0)))

(event `self.ReceiveTick`
  (params (DeltaSeconds :type "Float (single-precision)"))
  (bind _charactermovement (`self.CharacterMovement`))
  (if (or (`self.bIsAttacking`) (`self.bIsStunned`))
    (set `CharacterMovementComponent.MaxWalkSpeed` 0.0 _charactermovement)
    (else
      (set `CharacterMovementComponent.MaxWalkSpeed` 100.0 _charactermovement)))
  (`|AIMoveTo` self (0.0 0.0 0.0) (`self.Target`) 50.0
    (:`then`
      (if (<= (`KismetMathLibrary.Vector_Distance` (`self.K2_GetActorLocation`) (`self.K2_GetActorLocation` (`GameplayStatics.GetPlayerCharacter` 0))) 200.0)
        (if (and (!= (`self.bIsAttacking`) true) (!= (`self.bIsStunned`) true))
          (set `self.bIsAttacking` true)
          ;[1 1 1] Attacks player if possible
          (`GameplayStatics.PlaySoundAtLocation` "/Game/Sounds/NewFolder/Monster_Attack_Charge_Cue.Monster_Attack_Charge_Cue" (0.0 0.0 0.0) (struct) 1.0 1.0 0.0 null null null null)
          (`KismetSystemLibrary.Delay` 2.0)
          (`self.Attack`)
          (set `self.bIsAttacking` false))))))

(fn `GetStunned`)

(fn `UserConstructionScript`)