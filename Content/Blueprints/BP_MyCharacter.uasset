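; Player character Blueprint with cooldown-limited movement, camera yaw input and audio cues.
; BeginPlay adds one of two Enhanced Input mapping contexts to player 0 based on ControllerIndex; inputs call MoveHorizontal, MoveVertical and CameraYaw.
; Tick pins the audio listener to the root with a yaw offset, counts down the move cooldown and plays a one-shot wardrobe rattle whenever CanHide turns true.
; Trace-based footstep audio exists but is never called.
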(event `self.ReceiveTick`
  (params (DeltaSeconds :type "Float (single-precision)"))
  (`PlayerController.SetAudioListenerOverride` (`GameplayStatics.GetPlayerController` 0) (`self.RootComponent`) (0.0 0.0 0.0) (struct :`Pitch` 90.0))
  (set `self.MoveCooldown` (- (`self.MoveCooldown`) DeltaSeconds))
  (`|ExecutionSequence`
    (:`then_0`
      (if (`self.bCanHide`)
        (`/Engine/EditorBlueprintResources/StandardMacros.DoOnce` false :!label _label
          (:`Completed`
            (`GameplayStatics.PlaySoundAtLocation` "/Game/Sounds/Wardrobe_Rattle_Cue.Wardrobe_Rattle_Cue" (`self.HideSpotLocation`) (struct) 1.0 1.0 0.0 null null null null)))
        (else
          (goto _label :!via `Reset`))))))

(event `self.ReceiveBeginPlay`
  (bind _asplayer_controller (cast `PlayerController` (`GameplayStatics.GetPlayerController` 0)))
  (bind _returnvalue (pcsubsystem `EnhancedInputLocalPlayerSubsystem` _asplayer_controller))
  (`/Engine/EditorBlueprintResources/StandardMacros.IsValid` _returnvalue
    (:`Is Valid`
      (if (== (`self.ControllerIndex`) 0)
        (`EnhancedInputSubsystemInterface.AddMappingContext` _returnvalue "/Game/Inputs/InputMapContext/IMC_Test1.IMC_Test1" 0 (struct))
        (else
          (`EnhancedInputSubsystemInterface.AddMappingContext` _returnvalue "/Game/Inputs/InputMapContext/IMC_Test2.IMC_Test2" 0 (struct)))))))

(event `EnhancedInput|/Game/Inputs/CustomActions/IA_Rotate`
  (params (ActionValue :type "Float (double-precision)") (ElapsedSeconds :type "Float (double-precision)") (TriggeredSeconds :type "Float (double-precision)") (InputAction :type "InputAction Object Reference" :default "/Game/Inputs/CustomActions/IA_Rotate.IA_Rotate"))
  ;[1 1 1] CameraInput
  (:`Started`
    (`self.CameraYaw` ActionValue)))

(event `EnhancedInput|/Game/Inputs/CustomActions/IA_Move1`
  (params (ActionValue :type "Vector2D Structure") (ElapsedSeconds :type "Float (double-precision)") (TriggeredSeconds :type "Float (double-precision)") (InputAction :type "InputAction Object Reference" :default "/Game/Inputs/CustomActions/IA_Move1.IA_Move1"))
  ;[1 1 1] MovementInput
  (:`Triggered`
    (if (<= (`self.MoveCooldown`) 0.0)
      (`self.MoveHorizontal` ActionValue_X)
      (`self.MoveVertical` ActionValue_Y)
      (set `self.MoveCooldown` 0.3 :!label _label_2)))
  (:`Started`
    (`self.MoveHorizontal` ActionValue_X)
    (`self.MoveVertical` ActionValue_Y)
    (goto _label_2)))

(fn `PlayFootsteps`
  (bind _audio (`self.Audio`))
  (bind _finished (`self.TraceFootSteps`))
  (if _finished
    (`AudioComponent.SetSound` _audio "/Game/Sounds/Movement/Steps/WoodSteps.WoodSteps")
    (`AudioComponent.Play` _audio 0.0)))

(fn `TraceFootSteps`
  (returns (Finished :type Boolean))
  (bind _returnvalue (`self.K2_GetActorLocation`))
  (bind _capsulecomponent (`self.CapsuleComponent`))
  (bind (_x _y _z) (`KismetMathLibrary.BreakVector3f` _returnvalue))
  (bind (_outhit _returnvalue_2) (`KismetSystemLibrary.SphereTraceSingle` _returnvalue (`KismetMathLibrary.MakeVector` _x _y (- _z (`CapsuleComponent.GetScaledCapsuleHalfHeight` _capsulecomponent))) (`CapsuleComponent.GetScaledCapsuleRadius` _capsulecomponent) "TraceTypeQuery1"))
  (return _returnvalue_2))

(fn `UserConstructionScript`)