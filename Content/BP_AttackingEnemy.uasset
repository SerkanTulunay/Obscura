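; BP_AttackingEnemy is an enemy that slowly pursues the player character and starts an attack on reaching them.
; Each Tick it issues AIMoveTo unless attacking or stunned; arrival plays audio, waits, then checks stun and sphere overlap.
; The attack ends at a cast to BP_MyCharacter with no effect wired after it, and IsAttacking is never set here.
; GetStunned stops the audio and sets IsStunned, which nothing here clears.
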(event `self.ReceiveBeginPlay`
  (set `CharacterMovementComponent.MaxWalkSpeed` 1.0 (`self.CharacterMovement`))
  (set `self.Target` (`GameplayStatics.GetPlayerCharacter` 0)))

(event `self.ReceiveActorBeginOverlap`
  (params (OtherActor :type "Actor Object Reference")))

(event `self.ReceiveTick`
  (params (DeltaSeconds :type "Float (single-precision)"))
  (bind _returnvalue (`GameplayStatics.GetPlayerCharacter` 0))
  (if (and (!= (`self.IsAttacking`) true) (!= (`self.IsStunned`) true))
    (`|AIMoveTo` self (0.0 0.0 0.0) (`self.Target`)
      (:`OnSuccess`
        (if (and (!= (`self.IsAttacking`) true) (!= (`self.IsStunned`) true))
          ;[1 1 1] Attacks player if possible
          (`AudioComponent.Play` (`self.Audio`) 0.0)
          (`KismetSystemLibrary.Delay` 1.0)
          (if (and (!= (`self.IsStunned`) true) (`PrimitiveComponent.IsOverlappingActor` (`self.Sphere`) _returnvalue))
            (cast `/Game/Blueprints/BP_MyCharacter` _returnvalue)))))))

(fn `GetStunned`
  (set `self.IsStunned` true)
  (`AudioComponent.Stop` (`self.Audio`)))

(fn `UserConstructionScript`)